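; A kill-volume actor that detects when the player's ball falls off the map.
; On BeginPlay it caches the BallPlayerController, the player ball character and the PlatformAttachActorBP.
; When the Cube overlaps the ball, it tells the controller via PlayerFallenOffEvent.
; Overlaps by other actors in the attach actor's array only print a debug message that map parts are hitting the trigger.
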(event `self.ReceiveBeginPlay`
  (bind _asball_player_controller (cast `/Game/PRE/Blueprints/Pawn/Player/BallPlayerController` (`GameplayStatics.GetPlayerController` 0)))
  (set `self.BallPlayerControllerRef` _asball_player_controller)
  (bind _returnvalue (`GameplayStatics.GetActorOfClass` "/Game/PRE/Blueprints/Pawn/Player/PlayerBallCharacterBP.PlayerBallCharacterBP_C"))
  (set `self.PlayerBallCharacterRef` _returnvalue)
  (bind _returnvalue_2 (`GameplayStatics.GetActorOfClass` "/Game/PRE/Blueprints/Maps/Platform/PlatformAttachActorBP.PlatformAttachActorBP_C"))
  (set `self.AttachActor` _returnvalue_2))

(event `self.Cube.OnComponentBeginOverlap`
  (params (OverlappedComponent :type "PrimitiveComponent Object Reference") (OtherActor :type "Actor Object Reference") (OtherComp :type "PrimitiveComponent Object Reference") (OtherBodyIndex :type Integer) (bFromSweep :type Boolean) (SweepResult :type "HitResult Structure (by ref)"))
  (if (== OtherActor (`self.PlayerBallCharacterRef`))
    (`/Game/PRE/Blueprints/Pawn/Player/BallPlayerController.PlayerFallenOffEvent` (`self.BallPlayerControllerRef`))
    (else
      (for _array_element (`/Game/PRE/Blueprints/Maps/Platform/PlatformAttachActorBP.NewVar_0` (`self.AttachActor`))
        (if (== OtherActor _array_element)
          (`KismetSystemLibrary.PrintString` "Part Of map is Hitting Death Trigger!"))))))

(fn `UserConstructionScript`)