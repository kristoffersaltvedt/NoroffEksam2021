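; Spawn point actor for the player ball in platform maps, supplying a world location to the player ball character.
; Its construction script line-traces from ActualSpawm to TargetToSpawn and, unless the hit actor is the stored ball, lowers ActualSpawm by the hit distance, offset up by its bounds radius to rest on the surface.
; StartExecutingTheBallActor stores the ball and character references, then passes that location back through FinishedExecutingTheBallActor.
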(event `StartExecutingTheBallActor`
  (params (BallPawn :type "/Game/PRE/Blueprints/Pawn/Ball/BallPawnBP Object Reference") (PlayerBallCharactr :type "/Game/PRE/Blueprints/Pawn/Player/PlayerBallCharacterBP Object Reference"))
  (set `self.BallActor` BallPawn)
  (set `self.Player Ball Charactr` PlayerBallCharactr)
  (`/Game/PRE/Blueprints/Pawn/Player/PlayerBallCharacterBP.FinishedExecutingTheBallActor` (`self.Player Ball Charactr`) (`SceneComponent.K2_GetComponentLocation` (`self.ActualSpawm`))))

(fn `UserConstructionScript`
  (bind _outhit (`KismetSystemLibrary.LineTraceSingleByProfile` :`Start` (`SceneComponent.K2_GetComponentLocation` (`self.ActualSpawm`)) :`End` (`SceneComponent.K2_GetComponentLocation` (`self.TargetToSpawn`)) :`bTraceComplex` true :`TraceColor` (struct :`G` 1.0 :`B` 0.586126 :`A` 1.0) :`DrawTime` 20.0))
  (bind (_bblockinghit _binitialoverlap _time _distance _location _impactpoint _normal _impactnormal _physmat _hitactor) (`GameplayStatics.BreakHitResult` _outhit))
  (if (!= (`self.BallActor`) _hitactor)
    (`SceneComponent.K2_SetWorldLocation` (`self.ActualSpawm`) (`KismetMathLibrary.MakeVector` (.x (`SceneComponent.K2_GetComponentLocation` (`self.ActualSpawm`))) (.y (`SceneComponent.K2_GetComponentLocation` (`self.ActualSpawm`))) (+ (- (.z (`SceneComponent.K2_GetComponentLocation` (`self.ActualSpawm`))) _distance) (`.SphereRadius` (`KismetSystemLibrary.GetComponentBounds` (`self.ActualSpawm`))))) false false)))