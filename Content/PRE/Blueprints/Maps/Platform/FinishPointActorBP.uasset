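; Finish point actor for the platform map that notifies the player controller when the player's ball reaches it.
; On BeginPlay it caches the BallPlayerController and, after a short delay, the CollisionHitTrigger of the BallPawnBP found in the level.
; When its Plane component begins overlapping that exact trigger, it calls FinishLineEvent on the controller.
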(event `self.ReceiveBeginPlay`
  ;[1 1 1] Save Nessesary references to variables for later use
  (bind _asball_player_controller (cast `/Game/PRE/Blueprints/Pawn/Player/BallPlayerController` (`GameplayStatics.GetPlayerController` 0)))
  (set `self.BallPlayerControllerRef` _asball_player_controller)
  (`KismetSystemLibrary.Delay` 0.01)
  (bind _returnvalue (`GameplayStatics.GetActorOfClass` "/Game/PRE/Blueprints/Pawn/Ball/BallPawnBP.BallPawnBP_C"))
  (set `self.Collision Hit Trigger` (`/Game/PRE/Blueprints/Pawn/Ball/BallPawnBP.CollisionHitTrigger` _returnvalue)))

(event `self.Plane.OnComponentBeginOverlap`
  (params (OverlappedComponent :type "PrimitiveComponent Object Reference") (OtherActor :type "Actor Object Reference") (OtherComp :type "PrimitiveComponent Object Reference") (OtherBodyIndex :type Integer) (bFromSweep :type Boolean) (SweepResult :type "HitResult Structure (by ref)"))
  ;[1 1 1] Check If the HitTrigger belonging to the player Pawn (ball) Is overlapping To this Trigger sqhere
  (if (== OtherComp (`self.Collision Hit Trigger`))
    (`/Game/PRE/Blueprints/Pawn/Player/BallPlayerController.FinishLineEvent` (`self.BallPlayerControllerRef`))))

(fn `UserConstructionScript`)