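; Configurable static mesh actor Blueprint that takes its mesh and up to three materials from variables.
; The construction script assigns the input mesh to the StaticMesh component and always sets the first material slot.
; The second slot is set only if its material is valid, and the third only if both the second and third are valid.
; The event graph holds no active logic.
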(fn `UserConstructionScript`
  (`StaticMeshComponent.SetStaticMesh` (`self.StaticMesh`) (`self.InputMesh`))
  (`PrimitiveComponent.SetMaterial` (`self.StaticMesh`) 0 (`self.Input Material1`))
  (`/Engine/EditorBlueprintResources/StandardMacros.IsValid` (`self.Input Material2`)
    (:`Is Valid`
      (`PrimitiveComponent.SetMaterial` (`self.StaticMesh`) 1 (`self.Input Material2`))
      (`/Engine/EditorBlueprintResources/StandardMacros.IsValid` (`self.Input Material3`)
        (:`Is Valid`
          (`PrimitiveComponent.SetMaterial` (`self.StaticMesh`) 2 (`self.Input Material3`)))))))