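; SpectatePathBP is a spline path actor that drives a spectator fly-along when play begins.
; A timeline, sped up through its play rate, maps its track to distance along the spline, moving and rotating a sphere component to follow the path.
; When the timeline finishes, it tells the PlayerBallCharacterBP found in the level to smoothly transition out of spectating.
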(event `self.ReceiveBeginPlay`
  (`SceneComponent.K2_SetWorldLocation` (`self.Sphere`) (`SplineComponent.GetLocationAtSplinePoint` (`self.Spline`) 0 "World") false false)
  (`TimelineComponent.SetPlayRate` (`self.PlaySpectatorCamera`) 3.0)
  (bind _returnvalue (`GameplayStatics.GetActorOfClass` "/Game/PRE/Blueprints/Pawn/Player/PlayerBallCharacterBP.PlayerBallCharacterBP_C"))
  (bind (_direction _followtrack) (`Timeline|PlaySpectatorCamera` :!via `PlayFromStart`)
    (:`Update`
      (bind _returnvalue_2 (* (`SplineComponent.GetSplineLength` (`self.Spline`)) _followtrack))
      (`SceneComponent.K2_SetWorldLocationAndRotation` (`self.Sphere`) (`SplineComponent.GetLocationAtDistanceAlongSpline` (`self.Spline`) _returnvalue_2 "World") (`SplineComponent.GetRotationAtDistanceAlongSpline` (`self.Spline`) _returnvalue_2 "World") false false))
    (:`Finished`
      (`/Game/PRE/Blueprints/Pawn/Player/PlayerBallCharacterBP.SmoothTransitionFromSpectateToEnd` _returnvalue))))

(fn `UserConstructionScript`)